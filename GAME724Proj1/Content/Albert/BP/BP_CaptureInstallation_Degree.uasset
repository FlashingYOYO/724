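; BP_CaptureInstallation_Degree is a capture-and-launch installation that grabs the player's physics ball on overlap.
; BeginPlay binds to the RollyController's pawn update to cache the ball and plays a slowed timeline that spins a cylinder mesh.
; When that ball enters the capsule, it changes state, stops, snaps to the arrow and receives the launch strength plus an optional angular rotation limit around the actor's right vector.
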(event OnComponentBeginOverlap(Capsule)
  (params (OverlappedComponent :type Primitive%20Component%20Object%20Reference) (OtherActor :type Actor%20Object%20Reference) (OtherComp :type Primitive%20Component%20Object%20Reference) (OtherBodyIndex :type Integer) (bFromSweep :type Boolean) (SweepResult :type Hit%20Result%20Structure%20%28by%20ref%29))
  (bind _physics_ball (Variables|Ref|GetPhysics%20Ball))
  (if (== OtherActor _physics_ball)
    (Variables|/Game/OriginalAsset/RollingBP/Blueprints/PhysicsBallBP.PhysicsBallBP_C|SetBallState _physics_ball "NewEnumerator1")
    (Default|StopBallMovement _physics_ball)
    (Transformation|SetActorLocation _physics_ball (Transformation|GetWorldLocation (Variables|Default|GetArrow)) false false)
    (Variables|/Game/OriginalAsset/RollingBP/Blueprints/PhysicsBallBP.PhysicsBallBP_C|SetShootForce _physics_ball (Variables|Prop|GetLaunchStrength))
    (Default|SetRotateLimit _physics_ball (Transformation|GetActorRightVector) (Variables|Prop|GetRotAngle) (Variables|Prop|GetHasAngleLimit))))

(event Custom|UpdatePlayerPawn_Event
  (params (ThirdPerson :type BP%20Rolly%20Character%20Object%20Reference) (PhysicsBall :type Physics%20Ball%20BP%20Object%20Reference))
  (Variables|Ref|SetThird%20Person ThirdPerson)
  (Variables|Ref|SetPhysics%20Ball PhysicsBall))

(event EventBeginPlay
  (bind _asrolly_controller (CallFunction|BFLGetController))
  (bind _output_get (Variables|Ref|SetAs%20Rolly%20Controller _asrolly_controller))
  (EventDispatchers|AssignUpdatePlayerPawn _output_get (delegate Custom|UpdatePlayerPawn_Event))
  (Components|Timeline|SetPlayRate (Variables|Default|GetTimeline) 0.2)
  (bind _newtrack_0 (Timeline|Timeline Play)
    (:Update
      (Transformation|SetRelativeRotation (Variables|Default|GetpCylinder5) (Math|Rotator|MakeRotator 0.0 (* _newtrack_0 3.6e+02) 0.0) false false))))

(event Collision|EventActorBeginOverlap
  (params (OtherActor :type Actor%20Object%20Reference)))

(event EventTick
  (params (DeltaSeconds :type Float%20%28single-precision%29)))

(fn ConstructionScript)