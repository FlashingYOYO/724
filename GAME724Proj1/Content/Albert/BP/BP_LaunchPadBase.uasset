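; Launch pad base actor that flings the player's physics ball in an arc toward its TargetSpace component.
; It caches the current ball through the RollyController's UpdatePlayerPawn dispatcher.
; Ball overlap with the Box calls LaunchArc via a DoOnce, reset on end overlap.
; It also opens a Gate guarding a proximity check that changes the ball's linear damping near the target, though no Gate Enter is wired.
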(event OnComponentBeginOverlap(Box)
  (params (OverlappedComponent :type Primitive%20Component%20Object%20Reference) (OtherActor :type Actor%20Object%20Reference) (OtherComp :type Primitive%20Component%20Object%20Reference) (OtherBodyIndex :type Integer) (bFromSweep :type Boolean) (SweepResult :type Hit%20Result%20Structure%20%28by%20ref%29))
  (bind _physics_ball (Variables|Ref|GetPhysics%20Ball))
  (if (== OtherActor _physics_ball)
    (Utilities|FlowControl|DoOnce false
      (:Completed
        (Utilities|FlowControl|Sequence
          (:then_0
            (Utilities|FlowControl|Gate true :!label _label ; enters at Open
              (:Exit
                (Utilities|IsValid (Variables|Ref|GetPhysics%20Ball)
                  (:Is%20Valid
                    (if (<= (Math|Vector|Distance(Vector) (Transformation|GetActorLocation (Variables|Ref|GetPhysics%20Ball)) (Transformation|GetWorldLocation (Variables|Default|GetTargetSpace))) 2e+02)
                      (Default|ChangeLinearDamp (Variables|Ref|GetPhysics%20Ball))
                      (goto _label Close)))
                  (:Is%20Not%20Valid
                    (goto _label Close))))))
          (:then_1
            (Default|LaunchArc _physics_ball (Transformation|GetActorLocation _physics_ball) (Transformation|GetWorldLocation (Variables|Default|GetTargetSpace)) (Variables|Prop|GetSuggest%20Arc))))))))

(event OnComponentEndOverlap(Box)
  (params (OverlappedComponent :type Primitive%20Component%20Object%20Reference) (OtherActor :type Actor%20Object%20Reference) (OtherComp :type Primitive%20Component%20Object%20Reference) (OtherBodyIndex :type Integer))
  (bind _physics_ball (Variables|Ref|GetPhysics%20Ball))
  (if (== OtherActor (Variables|Ref|GetPhysics%20Ball))
    (Utilities|FlowControl|DoOnce false) ; enters at Reset
  ))

(event Custom|UpdatePlayerPawn_Event
  (params (ThirdPerson :type BP%20Rolly%20Character%20Object%20Reference) (PhysicsBall :type Physics%20Ball%20BP%20Object%20Reference))
  (Variables|Ref|SetThird%20Person ThirdPerson)
  (Variables|Ref|SetPhysics%20Ball PhysicsBall))

(event EventBeginPlay
  (bind _asrolly_controller (CallFunction|BFLGetController))
  (bind _output_get (Variables|Ref|SetAs%20Rolly%20Controller _asrolly_controller))
  (EventDispatchers|AssignUpdatePlayerPawn _output_get (delegate Custom|UpdatePlayerPawn_Event)))

(event Collision|EventActorBeginOverlap
  (params (OtherActor :type Actor%20Object%20Reference)))

(event EventTick
  (params (DeltaSeconds :type Float%20%28single-precision%29)))

(fn ConstructionScript)