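; BP_Gate is a gate that opens and closes automatically in an endless loop from BeginPlay.
; The loop calls DoorOpen and DoorClose in turn, separated by delays from CloseTime and Opentime.
; Each event plays its own timeline, which lerps the Door's relative location and rotation between closed and open values, with play rate hardcoded in the update.
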(event Custom|DoorOpen
  (bind _door (Variables|Default|GetDoor))
  (bind _newtrack_0 (Timeline|Timeline PlayFromStart)
    (:Update
      (Components|Timeline|SetPlayRate (Variables|Default|GetTimeline) 3.0)
      (Transformation|SetRelativeLocation _door (Math|Vector|Lerp(Vector) (Variables|Default|GetCloseLoc) (Variables|Default|GetOpenLoc) _newtrack_0) false false)
      (Transformation|SetRelativeRotation _door (Math|Rotator|Lerp(Rotator) (Variables|Default|GetCloseRot) (Variables|Default|GetOpenRot) _newtrack_0) false false))))

(event Custom|DoorClose
  (bind _door (Variables|Default|GetDoor))
  (bind _newtrack_0 (Timeline|Timeline_0 PlayFromStart)
    (:Update
      (Components|Timeline|SetPlayRate (Variables|Default|GetTimeline_0) 3.0)
      (Transformation|SetRelativeLocation _door (Math|Vector|Lerp(Vector) (Variables|Default|GetOpenLoc) (Variables|Default|GetCloseLoc) _newtrack_0) false false)
      (Transformation|SetRelativeRotation _door (Math|Rotator|Lerp(Rotator) (Variables|Default|GetOpenRot) (Variables|Default|GetCloseRot) _newtrack_0) false false))))

(event EventBeginPlay
  (CallFunction|DoorOpen :!label _label)
  (Utilities|FlowControl|Delay (Variables|Default|GetCloseTime))
  (CallFunction|DoorClose)
  (Utilities|FlowControl|Delay (Variables|Default|GetOpentime))
  (goto _label))

(fn ConstructionScript)