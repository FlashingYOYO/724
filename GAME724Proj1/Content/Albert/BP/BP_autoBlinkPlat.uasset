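; Auto-blinking platform actor that repeatedly vanishes and reappears on a timer.
; From BeginPlay, a Blink event hides the Cube and disables its collision for BlinkTime, then restores visibility and query-and-physics collision for Showntime.
; Blink then calls itself again, looping indefinitely through Delays without using Tick, so the platform always starts in the hidden phase.
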(event Custom|Blink
  (bind _cube (Variables|Default|GetCube))
  (bind _cube_2 (Variables|Default|GetCube))
  (Rendering|SetVisibility _cube_2 false false)
  (Collision|SetCollisionEnabled _cube_2 "NoCollision")
  (Utilities|FlowControl|Delay (Variables|Default|GetBlinkTime))
  (Rendering|SetVisibility _cube true false)
  (Collision|SetCollisionEnabled _cube "QueryAndPhysics")
  (Utilities|FlowControl|Delay (Variables|Default|GetShowntime))
  (CallFunction|Blink))

(event EventBeginPlay
  (CallFunction|Blink))

(event Collision|EventActorBeginOverlap
  (params (OtherActor :type Actor%20Object%20Reference)))

(event EventTick
  (params (DeltaSeconds :type Float%20%28single-precision%29)))

(fn ConstructionScript)