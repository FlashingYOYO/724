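; BP_SpeedPlatform_Base is a boost pad that pushes the player's physics ball along its arrow direction, scaled by PushStrength.
; It tracks the current player pawns through the controller's UpdatePlayerPawn dispatcher, so only that ball triggers the box overlap.
; Entering applies the impulse and plays a 2D speed sound, while the leave event is an empty hook.
; Activate and deactivate events toggle visibility and collision.
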(event OnComponentBeginOverlap(Box)
  (params (OverlappedComponent :type Primitive%20Component%20Object%20Reference) (OtherActor :type Actor%20Object%20Reference) (OtherComp :type Primitive%20Component%20Object%20Reference) (OtherBodyIndex :type Integer) (bFromSweep :type Boolean) (SweepResult :type Hit%20Result%20Structure%20%28by%20ref%29))
  (if (== OtherActor (Variables|Default|GetPhysics%20Ball))
    (CallFunction|CollisionEventR)
    (Audio|PlaySound2D "/Game/Albert/SFX/S_speed.S_speed" 1.0 1.0 0.0 0 0)))

(event OnComponentEndOverlap(Box)
  (params (OverlappedComponent :type Primitive%20Component%20Object%20Reference) (OtherActor :type Actor%20Object%20Reference) (OtherComp :type Primitive%20Component%20Object%20Reference) (OtherBodyIndex :type Integer))
  (if (== OtherActor (Variables|Default|GetPhysics%20Ball))
    (CallFunction|LeaveEventR)))

(event Custom|UpdatePlayerPawn_Event
  (params (ThirdPerson :type BP%20Rolly%20Character%20Object%20Reference) (PhysicsBall :type Physics%20Ball%20BP%20Object%20Reference))
  (Variables|Default|SetThird%20Person ThirdPerson)
  (Variables|Default|SetPhysics%20Ball PhysicsBall))

(event Custom|CollisionEvent_r
  (Default|ApplyImpulseforBall (Variables|Default|GetPhysics%20Ball) (* (Math|Vector|GetForwardVector (Variables|Default|GetArrow)) (Variables|Prop|GetPushStrength))))

(event Custom|LeaveEvent_r)

(event Custom|Deactivate%20Self
  (Rendering|SetVisibility (Variables|Default|GetDefaultSceneRoot) false true)
  (Collision|SetCollisionEnabled (Variables|Default|GetSpeedUp) "NoCollision"))

(event Custom|ActivateSelf
  (Rendering|SetVisibility (Variables|Default|GetDefaultSceneRoot) true true)
  (Collision|SetCollisionEnabled (Variables|Default|GetSpeedUp) "QueryAndPhysics")
  (Collision|SetCollisionEnabled (Variables|Default|GetBox) "QueryOnly"))

(event EventBeginPlay
  (bind _asbp_rolly_character (CallFunction|BFLGetThirdPerson))
  (Variables|Default|SetThird%20Person _asbp_rolly_character)
  (bind _asrolly_controller (CallFunction|BFLGetController))
  (EventDispatchers|AssignUpdatePlayerPawn _asrolly_controller (delegate Custom|UpdatePlayerPawn_Event)))

(event Collision|EventActorBeginOverlap
  (params (OtherActor :type Actor%20Object%20Reference)))

(event EventTick
  (params (DeltaSeconds :type Float%20%28single-precision%29)))

(fn ConstructionScript)