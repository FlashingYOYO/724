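; BP_SpeedPlatform1 is a toggleable speed-boost platform, apparently meant to push the physics ball.
; SetPlatformActive stores IsActive and switches both the SpeedUp component's visibility and the Box trigger's query-only collision on or off.
; Box overlap casts to PhysicsBallBP but does nothing further.
; The velocity-change impulse along the Arrow's forward vector, scaled by PushStrength, is disconnected, so no boost is applied.
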(event OnComponentBeginOverlap(Box)
  (params (OverlappedComponent :type Primitive%20Component%20Object%20Reference) (OtherActor :type Actor%20Object%20Reference) (OtherComp :type Primitive%20Component%20Object%20Reference) (OtherBodyIndex :type Integer) (bFromSweep :type Boolean) (SweepResult :type Hit%20Result%20Structure%20%28by%20ref%29))
  (bind _asphysics_ball_bp (Utilities|Casting|CastToPhysicsBallBP OtherActor)))

(event Custom|SetPlatformActive
  (params (NewActive :type Boolean))
  (Variables|Default|SetIsActive NewActive)
  (if (Variables|Default|GetIsActive)
    (Rendering|SetVisibility (Variables|Default|GetSpeedUp) true false)
    (Collision|SetCollisionEnabled (Variables|Default|GetBox) "QueryOnly")
    (else
      (Rendering|SetVisibility (Variables|Default|GetSpeedUp) false false)
      (Collision|SetCollisionEnabled (Variables|Default|GetBox) "NoCollision"))))

(event EventBeginPlay)

(event Collision|EventActorBeginOverlap
  (params (OtherActor :type Actor%20Object%20Reference)))

(event EventTick
  (params (DeltaSeconds :type Float%20%28single-precision%29)))

(fn ConstructionScript)