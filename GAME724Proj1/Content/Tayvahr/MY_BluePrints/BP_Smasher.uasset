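; BP_Smasher is a looping crusher hazard that calls ApplyDamage on whatever its Smasher component hits.
; From BeginPlay, the MoveSmasher event moves the component to DestinationTransform's location and rotation, waits, moves it back, waits again, then calls itself.
; The construction script places the Destination component at that same transform, and variables set the move duration and both waits.
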(event OnComponentHit(Smasher)
  (params (HitComponent :type Primitive%20Component%20Object%20Reference) (OtherActor :type Actor%20Object%20Reference) (OtherComp :type Primitive%20Component%20Object%20Reference) (NormalImpulse :type Vector :default "0, 0, 0") (Hit :type Hit%20Result%20Structure%20%28by%20ref%29))
  (Game|Damage|ApplyDamage OtherActor 0.0 0 0))

(event Custom|MoveSmasher
  (bind _destinationtransform (Variables|Default|GetDestinationTransform))
  (Components|MoveComponentTo (Variables|Default|GetSmasher) (.location _destinationtransform) (.rotation _destinationtransform) false false (Variables|Default|GetMovementSpeed) false)
  (Utilities|FlowControl|Delay (Variables|Default|GetWait%20Time))
  (Components|MoveComponentTo (Variables|Default|GetSmasher) "0, 0, 0" "0, 0, 0" false false (Variables|Default|GetMovementSpeed) false)
  (Utilities|FlowControl|Delay (Variables|Default|GetResetWaitTime))
  (CallFunction|MoveSmasher))

(event EventBeginPlay
  (CallFunction|MoveSmasher))

(fn ConstructionScript
  (Transformation|SetRelativeTransform (Variables|Default|GetDestination) (Variables|Default|GetDestinationTransform) false false))