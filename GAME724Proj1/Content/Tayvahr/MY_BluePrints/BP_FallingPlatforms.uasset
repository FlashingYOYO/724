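; BP_FallingPlatforms is a platform that moves when the player's BP_RollyCharacter overlaps its trigger box.
; The overlap calls MovePlatform, which uses MoveComponentTo to slide and rotate the Cube to DestinationTransform over Speed, used as the move duration.
; The construction script places the Destination component at that same transform to mark the end pose.
; The move is one-way, with no return logic.
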(event OnComponentBeginOverlap(Box)
  (params (OverlappedComponent :type Primitive%20Component%20Object%20Reference) (OtherActor :type Actor%20Object%20Reference) (OtherComp :type Primitive%20Component%20Object%20Reference) (OtherBodyIndex :type Integer) (bFromSweep :type Boolean) (SweepResult :type Hit%20Result%20Structure%20%28by%20ref%29))
  (Utilities|Casting|CastToBP_RollyCharacter OtherActor)
  (CallFunction|MovePlatform))

(event Custom|MovePlatform
  (bind _destination_transform (Variables|Default|GetDestination%20Transform))
  (Components|MoveComponentTo (Variables|Default|GetCube) (.location _destination_transform) (.rotation _destination_transform) false false (Variables|Default|GetSpeed) false))

(event EventBeginPlay)

(event Collision|EventActorBeginOverlap
  (params (OtherActor :type Actor%20Object%20Reference)))

(event EventTick
  (params (DeltaSeconds :type Float%20%28single-precision%29)))

(fn ConstructionScript
  (Transformation|SetRelativeTransform (Variables|Default|GetDestination) (Variables|Default|GetDestination%20Transform) false false))