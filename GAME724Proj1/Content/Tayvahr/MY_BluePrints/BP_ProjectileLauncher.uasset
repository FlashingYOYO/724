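; BP_ProjectileLauncher is an actor that fires one BP_Projectile on BeginPlay and again every 10 seconds through a delay loop.
; FireVolley moves Target to a random point in Box, then solves a debug-drawn high-arc toss from Spawn.
; The scaled toss velocity feeds the spawn, but the projectile's movement velocity is then overwritten straight up.
; The looping timer, projectile count loop and spread logic are unused.
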(event Custom|Fireit
  (CallFunction|FireVolley)
  (Utilities|FlowControl|Delay 1e+01)
  (CallFunction|Fireit))

(event EventBeginPlay
  (CallFunction|FireVolley)
  (Utilities|FlowControl|Delay 1e+01)
  (CallFunction|Fireit))

(fn ConstructionScript)

(fn FireVolley
  (bind _spawn (Variables|Default|Getspawn))
  (bind _box (Variables|Default|GetBox))
  (bind _returnvalue (Transformation|GetWorldTransform _spawn))
  (Transformation|SetRelativeLocation (Variables|Default|GetTarget) (Math|Random|RandomPointinBoundingBox (Variables|/Script/Engine.SceneComponent|GetRelativeLocation _box) (Variables|/Script/Engine.BoxComponent|GetBoxExtent _box)) false false)
  (bind _tossvelocity (Class|GameplayStatics|BlueprintSuggestProjectileVelocity (Transformation|GetWorldLocation (Variables|Default|Getspawn)) (Transformation|GetWorldLocation (Variables|Default|GetTarget)) 1e+03 0.0 "TraceFullPath" 0.0 true true true))
  (bind _returnvalue_2 (Game|SpawnActorfromClass "/Game/Tayvahr/MY_BluePrints/BP_Projectile.BP_Projectile_C" (Math|Transform|MakeTransform (.location _returnvalue) (.rotation _returnvalue) "1.000000,1.000000,1.000000") "Undefined" "MultiplyWithRoot" 0 (* _tossvelocity 1e+03) 0))
  (bind _asbp_projectile (Utilities|Casting|CastToBP_Projectile _returnvalue_2))
  (Variables|/Script/Engine.MovementComponent|SetVelocity (Variables|/Game/Tayvahr/MY_BluePrints/BP_Projectile.BP_Projectile_C|GetProjectileMovement _asbp_projectile) "0.000000,0.000000,50000.000000"))