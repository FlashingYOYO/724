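; BP_ProjectileTest is a test turret that repeatedly lobs volleys of BP_Projectile around the player's current pawn.
; On BeginPlay it caches the player and binds to the controller's pawn update to track ThirdPerson or PhysicsBall, then starts a looping TimeGap timer.
; Each tick of that timer spawns several projectiles at the Arrow, with custom-arc launch velocities solved from the actor's location.
; CalculateTheFireRange randomizes X and Y targets within RangeX of the pawn, at its height.
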(event Custom|UpdatePlayerPawn_Event
  (params (ThirdPerson :type BP%20Rolly%20Character%20Object%20Reference) (PhysicsBall :type Physics%20Ball%20BP%20Object%20Reference))
  (Variables|Ref|SetThird%20Person ThirdPerson)
  (Variables|Ref|SetPhysics%20Ball PhysicsBall))

(event Custom|FireTheBullet
  (for _index (range 0 3)
    (bind _outlaunchvelocity (Game|SuggestProjectileVelocityCustomArc (Transformation|GetActorLocation) (CallFunction|CalculatetheFireRange) 0.0 0.5))
    (Game|SpawnActorfromClass "/Game/Tayvahr/MY_BluePrints/BP_Projectile.BP_Projectile_C" (Math|Transform|MakeTransform (Transformation|GetWorldLocation (Variables|Default|GetArrow)) "0, 0, 0" "1.000000,1.000000,1.000000") "Undefined" "MultiplyWithRoot" 0 _outlaunchvelocity 0)))

(event EventBeginPlay
  (Utilities|FlowControl|Sequence
    (:then_0
      (bind _asrolly_controller (CallFunction|BFLGetController))
      (bind _output_get (Variables|Ref|SetAs%20Rolly%20Controller _asrolly_controller))
      (bind _asbp_rolly_character (CallFunction|BFLGetThirdPerson))
      (Variables|Ref|SetThird%20Person _asbp_rolly_character)
      (EventDispatchers|AssignUpdatePlayerPawn _output_get (delegate Custom|UpdatePlayerPawn_Event)))
    (:then_1
      (Utilities|Time|SetTimerbyEvent (delegate Custom|FireTheBullet) (Variables|Default|GetTimeGap) true))))

(event Collision|EventActorBeginOverlap
  (params (OtherActor :type Actor%20Object%20Reference)))

(event EventTick
  (params (DeltaSeconds :type Float%20%28single-precision%29)))

(fn ConstructionScript)

(fn CalculatetheFireRange
  (bind _returnvalue (Math|Random|RandomFloatinRange 0.0 3.6e+02))
  (bind _third_person (Variables|Ref|GetThird%20Person))
  (bind _rangex (Variables|Default|GetRangeX))
  (bind _third_person_2 (Variables|Ref|GetThird%20Person))
  (bind _physics_ball (Variables|Ref|GetPhysics%20Ball))
  (bind _returnvalue_2 (Utilities|IsValid _third_person))
  (bind _returnvalue_3 (Math|Random|RandomFloatinRange 0.0 _rangex))
  (bind _returnvalue_4 (select _returnvalue_2 _third_person_2 _physics_ball))
  (bind _returnvalue_5 (Transformation|GetActorLocation _returnvalue_4))
  (bind (_x _y _z) (Math|Vector|BreakVector _returnvalue_5))
  (return (Math|Vector|MakeVector (+ (* (Math|Trig|Cos(Degrees) _returnvalue) _returnvalue_3) _x) (+ (* (Math|Trig|Sin(Degrees) _returnvalue) _returnvalue_3) _y) _z)))