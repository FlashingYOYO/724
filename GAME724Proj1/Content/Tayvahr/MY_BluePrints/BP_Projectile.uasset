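; BP_Projectile is a moving projectile actor that knocks the player back on contact.
; Its construction script copies Velocity and InitialSpeed into ProjectileMovement, and BeginPlay sets a four-second lifespan with a matching delayed explosion sound.
; Overlapping a BP_RollyCharacter launches player 0 along a fixed world +X and upward vector, then destroys the projectile and plays the sound.
; The PhysicsBallBP overlap branch only casts, with no action.
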(event OnComponentBeginOverlap(Sphere)
  (params (OverlappedComponent :type Primitive%20Component%20Object%20Reference) (OtherActor :type Actor%20Object%20Reference) (OtherComp :type Primitive%20Component%20Object%20Reference) (OtherBodyIndex :type Integer) (bFromSweep :type Boolean) (SweepResult :type Hit%20Result%20Structure%20%28by%20ref%29))
  (Utilities|FlowControl|Sequence
    (:then_0
      (Utilities|Casting|CastToBP_RollyCharacter OtherActor)
      (Character|LaunchCharacter (Game|GetPlayerCharacter 0) "700.000000,0.000000,700.000000" true true)
      (Actor|DestroyActor)
      (Audio|PlaySoundatLocation "/Game/Tayvahr/MY_BluePrints/Sounds/ProjectileExplosion.ProjectileExplosion" (Transformation|GetWorldLocation (Variables|Default|GetSphere)) "0, 0, 0" 1.0 1.0 0.0 "/Game/Tayvahr/MY_BluePrints/Sounds/Smasher_Attenuation.Smasher_Attenuation" 0 0 0))
    (:then_1
      (Utilities|Casting|CastToPhysicsBallBP OtherActor))))

(event Custom|LifeSpan
  (Actor|SetLifeSpan 4.0)
  (Utilities|FlowControl|Delay 4.0)
  (Audio|PlaySoundatLocation "/Game/Tayvahr/MY_BluePrints/Sounds/ProjectileExplosion.ProjectileExplosion" (Transformation|GetWorldLocation (Variables|Default|GetSphere)) "0, 0, 0" 1.0 1.0 0.0 "/Game/Tayvahr/MY_BluePrints/Sounds/Smasher_Attenuation.Smasher_Attenuation" 0 0 0))

(event EventBeginPlay
  (CallFunction|LifeSpan))

(event Collision|EventActorBeginOverlap
  (params (OtherActor :type Actor%20Object%20Reference)))

(event EventTick
  (params (DeltaSeconds :type Float%20%28single-precision%29)))

(fn ConstructionScript
  (Variables|/Script/Engine.MovementComponent|SetVelocity (Variables|Default|GetProjectileMovement) (Variables|Default|GetVelocity))
  (Variables|/Script/Engine.ProjectileMovementComponent|SetInitialSpeed (Variables|Default|GetProjectileMovement) (Variables|Default|GetInitial%20Speed)))