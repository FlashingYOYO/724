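; BP_Mover is a moving platform that travels to a set destination and back once when play begins.
; MoveThePlatform uses MoveComponentTo to interpolate Platform to DestinationTransform's location and rotation over MoveSpeed, which acts as a duration.
; It waits WaitTime, moves back to the default relative target, then waits again, with no loop shown.
; The Construction Script places the Destination component at DestinationTransform, marking the endpoint.
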(event Custom|MoveThePlatform
  (bind _destinationtransform (Variables|Default|GetDestinationTransform))
  (Components|MoveComponentTo (Variables|Default|GetPlatform) (.location _destinationtransform) (.rotation _destinationtransform) false false (Variables|Default|GetMoveSpeed) false)
  (Utilities|FlowControl|Delay (Variables|Default|GetWaitTime))
  (Components|MoveComponentTo (Variables|Default|GetPlatform) "0, 0, 0" "0, 0, 0" false false (Variables|Default|GetMoveSpeed) false)
  (Utilities|FlowControl|Delay (Variables|Default|GetWaitTime)))

(event EventBeginPlay
  (CallFunction|MovethePlatform))

(fn ConstructionScript
  (Transformation|SetRelativeTransform (Variables|Default|GetDestination) (Variables|Default|GetDestinationTransform) false false))