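; BP_Projectile1 is a projectile actor that knocks the player character into the air.
; Its construction script copies its Velocity and InitialSpeed variables into the ProjectileMovement component, and BeginPlay gives it a limited lifespan.
; Any overlap on Sphere1 launches player 0's character along a fixed forward-and-up world vector, overriding current velocity, without checking which actor overlapped.
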(event OnComponentBeginOverlap(Sphere1)
  (params (OverlappedComponent :type Primitive%20Component%20Object%20Reference) (OtherActor :type Actor%20Object%20Reference) (OtherComp :type Primitive%20Component%20Object%20Reference) (OtherBodyIndex :type Integer) (bFromSweep :type Boolean) (SweepResult :type Hit%20Result%20Structure%20%28by%20ref%29))
  (Character|LaunchCharacter (Game|GetPlayerCharacter 0) "700.000000,0.000000,700.000000" true true))

(event EventBeginPlay
  (Actor|SetLifeSpan 1e+01))

(event Collision|EventActorBeginOverlap
  (params (OtherActor :type Actor%20Object%20Reference)))

(event EventTick
  (params (DeltaSeconds :type Float%20%28single-precision%29)))

(fn ConstructionScript
  (Variables|/Script/Engine.MovementComponent|SetVelocity (Variables|Default|GetProjectileMovement) (Variables|Default|GetVelocity))
  (Variables|/Script/Engine.ProjectileMovementComponent|SetInitialSpeed (Variables|Default|GetProjectileMovement) (Variables|Default|GetInitial%20Speed)))