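; BP_Accelerate_AllDirection is a boost trigger that accelerates the player's physics ball along whatever direction it is already moving.
; It binds to the Rolly controller's UpdatePlayerPawn dispatcher on BeginPlay to cache the current third-person pawn and physics ball references.
; When that cached ball begins overlapping the Box component, its current velocity is scaled by VelocityMul and set as the new velocity.
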(event OnComponentBeginOverlap(Box)
  (params (OverlappedComponent :type Primitive%20Component%20Object%20Reference) (OtherActor :type Actor%20Object%20Reference) (OtherComp :type Primitive%20Component%20Object%20Reference) (OtherBodyIndex :type Integer) (bFromSweep :type Boolean) (SweepResult :type Hit%20Result%20Structure%20%28by%20ref%29))
  (bind _physics_ball (Variables|Ref|GetPhysics%20Ball))
  (if (== OtherActor _physics_ball)
    (Default|SetNewVelocity _physics_ball (* (Transformation|GetVelocity _physics_ball) (Variables|Default|GetVelocityMul)))))

(event Custom|UpdatePlayerPawn_Event
  (params (ThirdPerson :type BP%20Rolly%20Character%20Object%20Reference) (PhysicsBall :type Physics%20Ball%20BP%20Object%20Reference))
  (Variables|Ref|SetThird%20Person ThirdPerson)
  (Variables|Ref|SetPhysics%20Ball PhysicsBall))

(event EventBeginPlay
  (bind _asrolly_controller (CallFunction|BFLGetController))
  (bind _output_get (Variables|Ref|SetAs%20Rolly%20Controller _asrolly_controller))
  (EventDispatchers|AssignUpdatePlayerPawn _output_get (delegate Custom|UpdatePlayerPawn_Event)))

(event Collision|EventActorBeginOverlap
  (params (OtherActor :type Actor%20Object%20Reference)))

(event EventTick
  (params (DeltaSeconds :type Float%20%28single-precision%29)))

(fn ConstructionScript)