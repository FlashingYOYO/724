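; BP_StartMenuController drives the start menu and the switch to level selection, apparently as a player controller.
; BeginPlay creates the WBP_StartMenu and WBP_LevelSelect widgets, adds only the start menu to the viewport and shows the mouse cursor.
; The GoLevelUI event removes the start menu and adds the pre-created level select widget, keeping the cursor visible.
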(event Custom|GoLevelUI
  (Widget|RemovefromParent (Variables|Default|GetStartMenu))
  (UserInterface|Viewport|AddtoViewport (Variables|Default|GetLevelSelect) 0)
  (Variables|Default|SetbShowMouseCursor true))

(event EventBeginPlay
  (bind _returnvalue (UserInterface|CreateWidget "/Game/Zxc/Blueprint/WBP/WBP_StartMenu.WBP_StartMenu_C"))
  (bind _output_get (Variables|Default|SetStartMenu _returnvalue))
  (UserInterface|Viewport|AddtoViewport _output_get 0)
  (bind _returnvalue_2 (UserInterface|CreateWidget "/Game/Zxc/Blueprint/WBP/WBP_LevelSelect.WBP_LevelSelect_C"))
  (Variables|Default|SetLevelSelect _returnvalue_2)
  (Variables|Default|SetbShowMouseCursor true))

(event EventTick
  (params (DeltaSeconds :type Float%20%28single-precision%29)))

(fn ConstructionScript)