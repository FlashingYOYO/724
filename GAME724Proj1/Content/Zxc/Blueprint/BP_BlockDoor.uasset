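; A door that only the player form matching its DoorType, physics ball or third-person human, can pass through.
; It binds to the Rolly controller's UpdatePlayerPawn dispatcher and toggles the mesh's collision off while the matching pawn is valid, on otherwise.
; A box trigger plays a sound when either pawn enters, using DoOnce gates to limit repeats.
; The construction script picks the door material from DoorType.
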(event OnComponentBeginOverlap(Box)
  (params (OverlappedComponent :type Primitive%20Component%20Object%20Reference) (OtherActor :type Actor%20Object%20Reference) (OtherComp :type Primitive%20Component%20Object%20Reference) (OtherBodyIndex :type Integer) (bFromSweep :type Boolean) (SweepResult :type Hit%20Result%20Structure%20%28by%20ref%29))
  (Utilities|FlowControl|Sequence
    (:then_0
      (if (== OtherActor (Variables|Default|GetPhysics%20Ball))
        (Utilities|FlowControl|DoOnce false
          (:Completed
            ;[1 0.9408 0 0.5] Sound
            (Audio|PlaySoundatLocation 0 (Transformation|GetActorLocation) "0, 0, 0" 1.0 1.0 0.0 0 0 0 0 :!label _label)))))
    (:then_1
      (if (== OtherActor (Variables|Default|GetThird%20Person))
        (Utilities|FlowControl|DoOnce false
          (:Completed
            (goto _label)))))))

(event OnComponentEndOverlap(Box)
  (params (OverlappedComponent :type Primitive%20Component%20Object%20Reference) (OtherActor :type Actor%20Object%20Reference) (OtherComp :type Primitive%20Component%20Object%20Reference) (OtherBodyIndex :type Integer))
  (Utilities|FlowControl|Sequence
    (:then_0
      (if (== OtherActor (Variables|Default|GetPhysics%20Ball))
        (Utilities|FlowControl|DoOnce false) ; enters at Reset
      ))
    (:then_1
      (if (== OtherActor (Variables|Default|GetThird%20Person))
        (Utilities|FlowControl|DoOnce false) ; enters at Reset
      ))))

(event Custom|UpdatePlayerPawn_Event
  (params (ThirdPerson :type BP%20Rolly%20Character%20Object%20Reference) (PhysicsBall :type Physics%20Ball%20BP%20Object%20Reference))
  (bind _staticmesh1 (Variables|Default|GetStaticMesh1))
  (Variables|Default|SetThird%20Person ThirdPerson)
  (Variables|Default|SetPhysics%20Ball PhysicsBall)
  (switch Utilities|FlowControl|Switch|SwitchonE_BlockDoorType (Variables|Default|GetDoorType)
    (:NewEnumerator0
      (Utilities|IsValid (Variables|Default|GetPhysics%20Ball)
        (:Is%20Valid
          (Collision|SetCollisionEnabled _staticmesh1 "NoCollision"))
        (:Is%20Not%20Valid
          (Collision|SetCollisionEnabled _staticmesh1 "QueryAndPhysics"))))
    (:NewEnumerator1
      (Utilities|IsValid (Variables|Default|GetThird%20Person)
        (:Is%20Valid
          (Collision|SetCollisionEnabled _staticmesh1 "NoCollision"))
        (:Is%20Not%20Valid
          (Collision|SetCollisionEnabled _staticmesh1 "QueryAndPhysics"))))))

(event EventBeginPlay
  (bind _asrolly_controller (CallFunction|BFLGetController))
  (bind _output_get (Variables|Default|SetAs%20Rolly%20Controller _asrolly_controller))
  (EventDispatchers|AssignUpdatePlayerPawn _output_get (delegate Custom|UpdatePlayerPawn_Event)))

(event Collision|EventActorBeginOverlap
  (params (OtherActor :type Actor%20Object%20Reference)))

(event EventTick
  (params (DeltaSeconds :type Float%20%28single-precision%29)))

(fn ConstructionScript
  (Rendering|Material|SetMaterial (Variables|Default|GetStaticMesh1) 0 (Utilities|Array|Get(acopy) (Variables|Default|GetDoorMat) (Math|Conversions|ToInteger(Byte) (Variables|Default|GetDoorType)))))