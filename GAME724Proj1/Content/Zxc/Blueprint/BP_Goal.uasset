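; BP_Goal is a level goal trigger that ends the run when the player's character or physics ball enters its Box.
; It caches the controller and character, refreshing both pawn references through the controller's UpdatePlayerPawn dispatcher.
; On overlap it disables input, hides the pawn, stops ball physics if needed, and plays a sound and Level Sequence.
; When the sequence finishes, it opens Map_Start.
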(event OnComponentBeginOverlap(Box)
  (params (OverlappedComponent :type Primitive%20Component%20Object%20Reference) (OtherActor :type Actor%20Object%20Reference) (OtherComp :type Primitive%20Component%20Object%20Reference) (OtherBodyIndex :type Integer) (bFromSweep :type Boolean) (SweepResult :type Hit%20Result%20Structure%20%28by%20ref%29))
  (bind _physics_ball (Variables|Default|GetPhysics%20Ball))
  (Utilities|FlowControl|Sequence
    (:then_0
      (if (== OtherActor _physics_ball)
        (Variables|Default|SetIsBallActive true)
        (Input|DisableInput (select (Variables|Default|GetIsBallActive) (Variables|Default|GetPhysics%20Ball) (Variables|Default|GetThird%20Person)) (Variables|Default|GetAs%20Rolly%20Controller) :!label _label)
        (if (Variables|Default|GetIsBallActive)
          (Physics|SetSimulatePhysics (Variables|/Game/OriginalAsset/RollingBP/Blueprints/PhysicsBallBP.PhysicsBallBP_C|GetBall _physics_ball) false))
        (Rendering|SetVisibility (Variables|/Script/Engine.Actor|GetRootComponent (select (Variables|Default|GetIsBallActive) (Variables|Default|GetPhysics%20Ball) (Variables|Default|GetThird%20Person))) false true)
        ;[1 0.9493 0 0.5] Sound
        (Audio|PlaySoundatLocation 0 (Transformation|GetActorLocation) "0, 0, 0" 1.0 1.0 0.0 0 0 0 0)
        (bind (_outactor _returnvalue) (Sequencer|Player|CreateLevelSequencePlayer (Variables|Default|GetLevel%20Sequence)))
        (Sequencer|Player|Play (Variables|/Script/LevelSequence.LevelSequenceActor|GetSequencePlayer _outactor) :!class /Script/MovieScene.MovieSceneSequencePlayer)
        (EventDispatchers|BindEventtoOnFinished _returnvalue (delegate Custom|ENDSequencer))))
    (:then_1
      (if (== OtherActor (Variables|Default|GetThird%20Person))
        (goto _label)))))

(event Custom|UpdatePlayerPawn_Event
  (params (ThirdPerson :type BP%20Rolly%20Character%20Object%20Reference) (PhysicsBall :type Physics%20Ball%20BP%20Object%20Reference))
  (Variables|Default|SetThird%20Person ThirdPerson)
  (Variables|Default|SetPhysics%20Ball PhysicsBall))

(event Custom|ENDSequencer
  (Game|OpenLevel(byName) "Map_Start"))

(event EventBeginPlay
  (bind _asrolly_controller (CallFunction|BFLGetController))
  (bind _output_get (Variables|Default|SetAs%20Rolly%20Controller _asrolly_controller))
  (bind _asbp_rolly_character (CallFunction|BFLGetThirdPerson))
  (Variables|Default|SetThird%20Person _asbp_rolly_character)
  (EventDispatchers|AssignUpdatePlayerPawn _output_get (delegate Custom|UpdatePlayerPawn_Event)))

(event Collision|EventActorBeginOverlap
  (params (OtherActor :type Actor%20Object%20Reference)))

(event EventTick
  (params (DeltaSeconds :type Float%20%28single-precision%29)))

(fn ConstructionScript)