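; Warning sign actor that follows the player's PhysicsBall pawn every tick and shows a timed sign effect.
; It binds to the Rolly controller's pawn updates, hiding the sign when a ThirdPerson pawn is valid, otherwise registering itself on the ball.
; ShowSign plays a timeline scaled to the given duration, driving the Alpha parameter of the MPC_SignInfo material parameter collection.
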(event Custom|ShowSign
  (params (Time :type Float%20%28double-precision%29))
  (Components|Timeline|SetPlayRate (Variables|Default|GetTimeline) (/ 1.0 Time))
  (bind _newtrack_0 (Timeline|Timeline PlayFromStart)
    (:Update
      (Rendering|Material|SetScalarParameterValue "/Game/Zxc/Material/MPC_SignInfo.MPC_SignInfo" "Alpha" _newtrack_0 :!class /Script/Engine.KismetMaterialLibrary))))

(event Custom|UpdatePlayerPawn_Event
  (params (ThirdPerson :type BP%20Rolly%20Character%20Object%20Reference) (PhysicsBall :type Physics%20Ball%20BP%20Object%20Reference))
  (Variables|Default|SetThird%20Person ThirdPerson)
  (bind _output_get (Variables|Default|SetPhysics%20Ball PhysicsBall))
  (Utilities|IsValid (Variables|Default|GetThird%20Person)
    (:Is%20Valid
      (Audio|Components|Audio|Stop (Variables|Default|GetTimeline))
      (Rendering|Material|SetScalarParameterValue "/Game/Zxc/Material/MPC_SignInfo.MPC_SignInfo" "Alpha" 0.0 :!class /Script/Engine.KismetMaterialLibrary))
    (:Is%20Not%20Valid
      (Variables|/Game/OriginalAsset/RollingBP/Blueprints/PhysicsBallBP.PhysicsBallBP_C|SetWarningSign _output_get self))))

(event EventBeginPlay
  (bind _asrolly_controller (CallFunction|BFLGetController))
  (bind _output_get (Variables|Default|SetAs%20Rolly%20Controller _asrolly_controller))
  (EventDispatchers|AssignUpdatePlayerPawn _output_get (delegate Custom|UpdatePlayerPawn_Event)))

(event Collision|EventActorBeginOverlap
  (params (OtherActor :type Actor%20Object%20Reference)))

(event EventTick
  (params (DeltaSeconds :type Float%20%28single-precision%29))
  (bind _physics_ball (Variables|Default|GetPhysics%20Ball))
  (Utilities|IsValid _physics_ball
    (:Is%20Valid
      (Transformation|SetActorLocation (Transformation|GetActorLocation _physics_ball) false false))))

(fn ConstructionScript)