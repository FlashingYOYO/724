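; Gravity field platform that redirects the player PhysicsBall's gravity along its Arrow when the ball enters the box, damping its velocity with a counter-impulse.
; If CanDisappear is set, a ball hit fades the cube through a dynamic material, disables collision, then restores it on a timer.
; The construction script fits cube and trigger to Size.
; Gravity reset on exit and respawn-event binding exist only as unconnected logic.
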(event OnComponentHit(Cube)
  (params (HitComponent :type Primitive%20Component%20Object%20Reference) (OtherActor :type Actor%20Object%20Reference) (OtherComp :type Primitive%20Component%20Object%20Reference) (NormalImpulse :type Vector :default "0, 0, 0") (Hit :type Hit%20Result%20Structure%20%28by%20ref%29))
  (if (Variables|Prop|GetCanDisappear)
    (if (== OtherActor (Variables|Ref|GetPhysics%20Ball))
      (Utilities|FlowControl|DoOnce false
        (:Completed
          (Components|Timeline|SetPlayRate (Variables|Default|GetTL_Fade) (/ 1.0 (Variables|Prop|GetFadeTime)))
          (bind _newtrack_0 (Timeline|TL_Fade PlayFromStart)
            (:Update
              (Rendering|Material|SetScalarParameterValue (Variables|Ref|GetDMI) "Phase" _newtrack_0 :!class /Script/Engine.MaterialInstanceDynamic))
            (:Finished
              (Collision|SetCollisionEnabled (Variables|Default|GetCube) "NoCollision")
              (bind _returnvalue (Utilities|Time|SetTimerbyEvent (delegate Custom|Appear) (Variables|Prop|GetTimeToAppear)))
              (Variables|Default|SetIterator _returnvalue))))))))

(event OnComponentBeginOverlap(Box)
  (params (OverlappedComponent :type Primitive%20Component%20Object%20Reference) (OtherActor :type Actor%20Object%20Reference) (OtherComp :type Primitive%20Component%20Object%20Reference) (OtherBodyIndex :type Integer) (bFromSweep :type Boolean) (SweepResult :type Hit%20Result%20Structure%20%28by%20ref%29))
  (bind _physics_ball (Variables|Ref|GetPhysics%20Ball))
  (bind _physics_ball_2 (Variables|Ref|GetPhysics%20Ball))
  (bind _arrow (Variables|Default|GetArrow))
  (bind _returnvalue (Math|Vector|GetForwardVector _arrow))
  (bind _returnvalue_2 (* _returnvalue 9.8e+02))
  (if (== OtherActor _physics_ball_2)
    (Default|ApplyImpulseforBall _physics_ball_2 (* (Variables|/Game/OriginalAsset/RollingBP/Blueprints/PhysicsBallBP.PhysicsBallBP_C|GetCurVeloctiy _physics_ball_2) -0.4))
    (Utilities|IsValid _physics_ball
      (:Is%20Valid
        (Default|ChangeGravityDirection _physics_ball _returnvalue_2)
        (Development|PrintString (Utilities|String|ToString(Vector) _returnvalue_2) true true "(R=0.000000,G=0.660000,B=1.000000,A=1.000000)" 2.0 "1")))))

(event OnComponentEndOverlap(Box)
  (params (OverlappedComponent :type Primitive%20Component%20Object%20Reference) (OtherActor :type Actor%20Object%20Reference) (OtherComp :type Primitive%20Component%20Object%20Reference) (OtherBodyIndex :type Integer)))

(event Custom|UpdatePlayerPawn_Event
  (params (ThirdPerson :type BP%20Rolly%20Character%20Object%20Reference) (PhysicsBall :type Physics%20Ball%20BP%20Object%20Reference))
  (bind _output_get (Variables|Ref|SetThird%20Person ThirdPerson))
  (bind _output_get_2 (Variables|Ref|SetPhysics%20Ball PhysicsBall)))

(event Custom|Appear
  (Collision|SetCollisionEnabled (Variables|Default|GetCube) "QueryAndPhysics")
  (Rendering|Material|SetScalarParameterValue (Variables|Ref|GetDMI) "Phase" 1.0 :!class /Script/Engine.MaterialInstanceDynamic)
  (Utilities|FlowControl|DoOnce false) ; enters at Reset
)

(event Custom|RespawnEvent_Event
  (Utilities|Time|ClearandInvalidateTimerbyHandle (Variables|Default|GetIterator))
  (Collision|SetCollisionEnabled (Variables|Default|GetCube) "QueryAndPhysics")
  (Rendering|Material|SetScalarParameterValue (Variables|Ref|GetDMI) "Phase" 1.0 :!class /Script/Engine.MaterialInstanceDynamic))

(event EventBeginPlay
  (Utilities|FlowControl|Sequence
    (:then_0
      (bind _asbp_rolly_character (CallFunction|BFLGetThirdPerson))
      (Variables|Ref|SetThird%20Person _asbp_rolly_character)
      (bind _asrolly_controller (CallFunction|BFLGetController))
      (bind _output_get (Variables|Ref|SetAs%20Rolly%20Controller _asrolly_controller))
      (EventDispatchers|AssignUpdatePlayerPawn _output_get (delegate Custom|UpdatePlayerPawn_Event)))
    (:then_1
      (bind _returnvalue (Rendering|Material|CreateDynamicMaterialInstance (Variables|Default|GetCube) 0 0 "None" :!class /Script/Engine.PrimitiveComponent))
      (Variables|Ref|SetDMI _returnvalue))))

(event Collision|EventActorBeginOverlap
  (params (OtherActor :type Actor%20Object%20Reference)))

(event EventTick
  (params (DeltaSeconds :type Float%20%28single-precision%29)))

(fn ConstructionScript
  (bind _size (Variables|Prop|GetSize))
  (bind _box (Variables|Default|GetBox))
  (bind (_x _y) (Math|Vector|BreakVector _size))
  (bind _returnvalue (* _size 5e+01))
  (Transformation|SetRelativeScale3D (Variables|Default|GetCube) (Math|Vector|MakeVector _x _y 0.2))
  (Components|Box|SetBoxExtent _box _returnvalue true)
  (Transformation|SetRelativeLocation _box (Math|Vector|MakeVector 0.0 0.0 (.Z (Math|Vector|BreakVector _returnvalue))) false false))