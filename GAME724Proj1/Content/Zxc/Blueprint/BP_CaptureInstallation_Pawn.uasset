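; Capture installation pawn that catches the player's physics ball and lets the player aim and launch it like a cannon.
; On capsule overlap it stops the ball, pins it to an arrow and has the Rolly controller switch to the capture camera; look input rotates the pawn.
; Holding shoot charges a material progress bar; release or full charge destroys the ball and passes a launch velocity to the controller's ball-camera switch.
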(event OnComponentBeginOverlap(Capsule)
  (params (OverlappedComponent :type Primitive%20Component%20Object%20Reference) (OtherActor :type Actor%20Object%20Reference) (OtherComp :type Primitive%20Component%20Object%20Reference) (OtherBodyIndex :type Integer) (bFromSweep :type Boolean) (SweepResult :type Hit%20Result%20Structure%20%28by%20ref%29))
  (bind _dmi (Variables|Ref|GetDMI))
  (bind _physics_ball (Variables|Ref|GetPhysics%20Ball))
  (if (== OtherActor _physics_ball)
    (Utilities|FlowControl|Sequence
      (:then_0
        (Rendering|Material|SetScalarParameterValue (Variables|Default|GetDMI_04) "TargetArmLength" (Variables|Default|GetTarget%20Arm%20Length) :!class /Script/Engine.MaterialInstanceDynamic))
      (:then_1
        (Variables|/Game/OriginalAsset/RollingBP/Blueprints/PhysicsBallBP.PhysicsBallBP_C|SetBallState _physics_ball "NewEnumerator1")
        (Default|StopBallMovement _physics_ball)
        (Transformation|SetActorLocation _physics_ball (Transformation|GetWorldLocation (Variables|Default|GetArrow)) false false)
        (Variables|/Game/OriginalAsset/RollingBP/Blueprints/PhysicsBallBP.PhysicsBallBP_C|SetShootForce _physics_ball (Variables|Prop|GetLaunchStrength))
        (Default|SwitchtoCaptureCamera (Variables|Ref|GetAs%20Rolly%20Controller) self _physics_ball)
        (Utilities|FlowControl|Gate true) ; enters at Open
      )
      (:then_2
        (Utilities|FlowControl|DoOnce false) ; enters at Reset
      ))))

(event Custom|UpdatePlayerPawn_Event
  (params (ThirdPerson :type BP%20Rolly%20Character%20Object%20Reference) (PhysicsBall :type Physics%20Ball%20BP%20Object%20Reference))
  (Variables|Ref|SetThird%20Person ThirdPerson)
  (Variables|Ref|SetPhysics%20Ball PhysicsBall))

(event Input|EnhancedActionEvents|EnhancedInputActionIA_Look
  (params (ActionValue :type Vector%202D%20Structure) (ElapsedSeconds :type Float%20%28double-precision%29) (TriggeredSeconds :type Float%20%28double-precision%29) (InputAction :type Input%20Action%20Object%20Reference :default "/Game/OriginalAsset/RollingBP/Input/Actions/IA_Look.IA_Look"))
  (Pawn|Input|AddControllerYawInput (.x ActionValue))
  (Pawn|Input|AddControllerPitchInput (.y ActionValue))
  (Transformation|SetActorRotation (Math|Rotator|MakeRotfromX (Math|Vector|GetForwardVector (Variables|Default|GetCamera)))))

(event Input|EnhancedActionEvents|EnhancedInputActionIA_Shoot
  (params (ActionValue :type Boolean) (ElapsedSeconds :type Float%20%28double-precision%29) (TriggeredSeconds :type Float%20%28double-precision%29) (InputAction :type Input%20Action%20Object%20Reference :default "/Game/OriginalAsset/RollingBP/Input/Actions/IA_Shoot.IA_Shoot"))
  (bind _dmi (Variables|Ref|GetDMI))
  (:Triggered
    (Utilities|FlowControl|Gate true :!label _label
      (:Exit
        (bind _output_get (Variables|Default|SetProgressBarPhase (Math|Float|Clamp(Float) (+ (Variables|Default|GetProgressBarPhase) (Utilities|Time|GetWorldDeltaSeconds)) 0.0 3.0)))
        (Rendering|Material|SetScalarParameterValue (Variables|Ref|GetDMI) "Phase" _output_get :!class /Script/Engine.MaterialInstanceDynamic)
        (if (>= (Variables|Default|GetProgressBarPhase) 3.0)
          (Utilities|FlowControl|DoOnce false
            (:Completed
              (Utilities|FlowControl|Sequence
                (:then_0
                  (Utilities|FlowControl|Gate true) ; enters at Close
                )
                (:then_1
                  (goto _label Close))
                (:then_2
                  (Actor|DestroyActor (Variables|Ref|GetPhysics%20Ball) :!label _label_2)
                  (Default|SwitchtoBallCamera (Variables|Ref|GetAs%20Rolly%20Controller) (* (Transformation|GetActorForwardVector) (* (Variables|Prop|GetLaunchStrength) (Math|Float|Clamp(Float) (Variables|Default|GetProgressBarPhase)))) (Transformation|GetActorTransform))
                  (Transformation|SetActorRotation (Variables|Default|GetInitRotation))
                  (Rendering|Material|SetScalarParameterValue _dmi "Alpha" 0.0 :!class /Script/Engine.MaterialInstanceDynamic)
                  (Variables|Default|SetProgressBarPhase 0.0)
                  (Rendering|Material|SetScalarParameterValue _dmi "Phase" 0.0 :!class /Script/Engine.MaterialInstanceDynamic)))))))))
  (:Started
    (Rendering|Material|SetScalarParameterValue (Variables|Ref|GetDMI) "Alpha" 1.0 :!class /Script/Engine.MaterialInstanceDynamic))
  (:Completed
    (Utilities|FlowControl|Sequence
      (:then_0
        (Utilities|FlowControl|Gate true) ; enters at Close
      )
      (:then_1
        (goto _label Close))
      (:then_2
        (goto _label_2)))))

(event EventBeginPlay
  (Utilities|FlowControl|Sequence
    (:then_0
      (bind _asrolly_controller (CallFunction|BFLGetController))
      (bind _output_get (Variables|Ref|SetAs%20Rolly%20Controller _asrolly_controller))
      (EventDispatchers|AssignUpdatePlayerPawn _output_get (delegate Custom|UpdatePlayerPawn_Event)))
    (:then_1
      (Variables|Default|SetInitRotation (Transformation|GetActorRotation))
      (Variables|Default|SetInitForward (Transformation|GetActorForwardVector)))
    (:then_2
      (bind _returnvalue (Rendering|Material|CreateDynamicMaterialInstance (Variables|Default|GetPlane) 0 0 "None" :!class /Script/Engine.PrimitiveComponent))
      (Variables|Ref|SetDMI _returnvalue)
      (bind _returnvalue_2 (Rendering|Material|CreateDynamicMaterialInstance (Variables|Default|GetpCylinder4) 0 0 "None" :!class /Script/Engine.PrimitiveComponent))
      (Variables|Default|SetDMI_04 _returnvalue_2)
      (bind _returnvalue_3 (Rendering|Material|CreateDynamicMaterialInstance (Variables|Default|GetpCylinder5) 0 0 "None" :!class /Script/Engine.PrimitiveComponent))
      (Variables|Default|SetDMI_05 _returnvalue_3))))

(event EventTick
  (params (DeltaSeconds :type Float%20%28single-precision%29))
  (bind _dmi (Variables|Ref|GetDMI))
  (Utilities|FlowControl|Sequence
    (:then_0
      (Utilities|FlowControl|Gate true
        (:Exit
          (Transformation|SetActorLocation (Variables|Ref|GetPhysics%20Ball) (Transformation|GetWorldLocation (Variables|Default|GetArrow)) false false))))
    (:then_1
      (Utilities|FlowControl|Gate true) ; enters at Open
    )))

(fn ConstructionScript
  (Variables|/Script/Engine.SpringArmComponent|SetTargetArmLength (Variables|Default|GetSpringArm) (Variables|Default|GetTarget%20Arm%20Length)))

(fn CalculateAngle
  (return (/ (Variables|Prop|GetAngleLimit) (Class|KismetMathLibrary|DegAcos (Math|Vector|DotProduct (Variables|Default|GetInitForward) (Transformation|GetActorForwardVector))))))