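; BP_CheckPoint is a checkpoint actor that registers itself as the last checkpoint of the third-person character or physics ball overlapping its box.
; It gets the third-person pawn on BeginPlay and refreshes both pawn references through the Rolly controller's UpdatePlayerPawn dispatcher.
; A new activation plays a sound while a timeline cross-fades the "Phase" dynamic material parameter from the previous checkpoint to this one, or sets it instantly if none exists.
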(event OnComponentBeginOverlap(Box)
  (params (OverlappedComponent :type Primitive%20Component%20Object%20Reference) (OtherActor :type Actor%20Object%20Reference) (OtherComp :type Primitive%20Component%20Object%20Reference) (OtherBodyIndex :type Integer) (bFromSweep :type Boolean) (SweepResult :type Hit%20Result%20Structure%20%28by%20ref%29))
  (bind _physics_ball (Variables|Ref|GetPhysics%20Ball))
  (bind _third_person (Variables|Ref|GetThird%20Person))
  (Utilities|FlowControl|Sequence
    (:then_0
      (if (== OtherActor _physics_ball)
        (if (not (== self (Variables|/Game/OriginalAsset/RollingBP/Blueprints/PhysicsBallBP.PhysicsBallBP_C|GetLastCheckPoint _physics_ball)))
          (CallFunction|GoFade (Variables|/Game/OriginalAsset/RollingBP/Blueprints/PhysicsBallBP.PhysicsBallBP_C|GetLastCheckPoint _physics_ball))
          (Variables|/Game/OriginalAsset/RollingBP/Blueprints/PhysicsBallBP.PhysicsBallBP_C|SetLastCheckPoint _physics_ball self)
          ;[1 0.9864 0 0.5] Sound
          (Audio|PlaySoundatLocation "/Game/Albert/SFX/S_checkPoint.S_checkPoint" (Transformation|GetActorLocation) "0, 0, 0" 1.0 1.0 0.0 0 0 0 0))))
    (:then_1
      (if (== OtherActor _third_person)
        (if (not (== (Variables|/Game/OriginalAsset/RollingBP/Blueprints/BP_RollyCharacter.BP_RollyCharacter_C|GetLastCheckPoint _third_person) self))
          (CallFunction|GoFade (Variables|/Game/OriginalAsset/RollingBP/Blueprints/BP_RollyCharacter.BP_RollyCharacter_C|GetLastCheckPoint _third_person))
          (Variables|/Game/OriginalAsset/RollingBP/Blueprints/BP_RollyCharacter.BP_RollyCharacter_C|SetLastCheckPoint _third_person self)
          (Audio|PlaySoundatLocation "/Game/Albert/SFX/S_checkPoint.S_checkPoint" (Transformation|GetActorLocation) "0, 0, 0" 1.0 1.0 0.0 0 0 0 0))))))

(event Custom|UpdatePlayerPawn_Event
  (params (ThirdPerson :type BP%20Rolly%20Character%20Object%20Reference) (PhysicsBall :type Physics%20Ball%20BP%20Object%20Reference))
  (Variables|Ref|SetThird%20Person ThirdPerson)
  (Variables|Ref|SetPhysics%20Ball PhysicsBall))

(event Custom|GoFade
  (params (LastCheckPoint :type BP%20Check%20Point%20Object%20Reference))
  (Utilities|IsValid LastCheckPoint
    (:Is%20Valid
      (bind _newtrack_0 (Timeline|TL PlayFromStart)
        (:Update
          (Rendering|Material|SetScalarParameterValue (Variables|BP_CheckPoint_C|GetDMI LastCheckPoint) "Phase" (- 1.0 _newtrack_0) :!class /Script/Engine.MaterialInstanceDynamic)
          (Rendering|Material|SetScalarParameterValue (Variables|Default|GetDMI) "Phase" _newtrack_0 :!class /Script/Engine.MaterialInstanceDynamic))))
    (:Is%20Not%20Valid
      (Rendering|Material|SetScalarParameterValue (Variables|Default|GetDMI) "Phase" 1.0 :!class /Script/Engine.MaterialInstanceDynamic))))

(event EventBeginPlay
  (Utilities|FlowControl|Sequence
    (:then_0
      (bind _asrolly_controller (CallFunction|BFLGetController))
      (bind _output_get (Variables|Ref|SetAs%20Rolly%20Controller _asrolly_controller))
      (EventDispatchers|AssignUpdatePlayerPawn _output_get (delegate Custom|UpdatePlayerPawn_Event)))
    (:then_1
      (bind _returnvalue (Rendering|Material|CreateDynamicMaterialInstance (Variables|Default|GetCube) 0 0 "None" :!class /Script/Engine.PrimitiveComponent))
      (Variables|Default|SetDMI _returnvalue))
    (:then_2
      (bind _asbp_rolly_character (CallFunction|BFLGetThirdPerson))
      (Variables|Ref|SetThird%20Person _asbp_rolly_character))))

(fn ConstructionScript)