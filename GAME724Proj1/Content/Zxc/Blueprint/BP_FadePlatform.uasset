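; Platform that fades out and loses collision after the player's physics ball hits it, then reappears after a delay, if CanDisappear is enabled.
; A DoOnce-gated timeline, scaled by FadeTime, drives the dynamic material's Phase parameter, and a timer restores the platform.
; The controller's UpdatePlayerPawn event refreshes the ball reference and restores the platform.
; The construction script picks the material from CanDisappear.
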(event OnComponentHit(Cube)
  (params (HitComponent :type Primitive%20Component%20Object%20Reference) (OtherActor :type Actor%20Object%20Reference) (OtherComp :type Primitive%20Component%20Object%20Reference) (NormalImpulse :type Vector :default "0, 0, 0") (Hit :type Hit%20Result%20Structure%20%28by%20ref%29))
  (if (Variables|Prop|GetCanDisappear)
    (if (== OtherActor (Variables|Ref|GetPhysics%20Ball))
      (Utilities|FlowControl|DoOnce false
        (:Completed
          (Components|Timeline|SetPlayRate (Variables|Default|GetTL_Fade) (/ 1.0 (Variables|Prop|GetFadeTime)))
          (bind _newtrack_0 (Timeline|TL_Fade PlayFromStart)
            (:Update
              (Rendering|Material|SetScalarParameterValue (Variables|Ref|GetDMI) "Phase" _newtrack_0 :!class /Script/Engine.MaterialInstanceDynamic))
            (:Finished
              (Collision|SetCollisionEnabled (Variables|Default|GetCube) "NoCollision")
              (bind _returnvalue (Utilities|Time|SetTimerbyEvent (delegate Custom|Appear) (Variables|Prop|GetTimeToAppear)))
              (Variables|Default|SetIterator _returnvalue))))))))

(event Custom|UpdatePlayerPawn_Event
  (params (ThirdPerson :type BP%20Rolly%20Character%20Object%20Reference) (PhysicsBall :type Physics%20Ball%20BP%20Object%20Reference))
  (Variables|Ref|SetAs%20BP%20Rolly%20Character ThirdPerson)
  (Variables|Ref|SetPhysics%20Ball PhysicsBall)
  (Utilities|IsValid (Variables|Ref|GetAs%20Rolly%20Controller)
    (:Is%20Valid
      (Audio|Components|Audio|Stop (Variables|Default|GetTL_Fade))
      (Rendering|Material|SetScalarParameterValue (Variables|Ref|GetDMI) "Phase" 1.0 :!class /Script/Engine.MaterialInstanceDynamic)
      (Collision|SetCollisionEnabled (Variables|Default|GetCube) "QueryAndPhysics")
      (Utilities|FlowControl|DoOnce false) ; enters at Reset
    )))

(event Custom|Appear
  (Collision|SetCollisionEnabled (Variables|Default|GetCube) "QueryAndPhysics")
  (Rendering|Material|SetScalarParameterValue (Variables|Ref|GetDMI) "Phase" 1.0 :!class /Script/Engine.MaterialInstanceDynamic)
  (Utilities|FlowControl|DoOnce false) ; enters at Reset
)

(event EventBeginPlay
  (Utilities|FlowControl|Sequence
    (:then_0
      (bind _asbp_rolly_character (CallFunction|BFLGetThirdPerson))
      (Variables|Ref|SetAs%20BP%20Rolly%20Character _asbp_rolly_character)
      (bind _asrolly_controller (CallFunction|BFLGetController))
      (bind _output_get (Variables|Ref|SetAs%20Rolly%20Controller _asrolly_controller))
      (EventDispatchers|AssignUpdatePlayerPawn _output_get (delegate Custom|UpdatePlayerPawn_Event)))
    (:then_1
      (bind _returnvalue (Rendering|Material|CreateDynamicMaterialInstance (Variables|Default|GetCube) 0 0 "None" :!class /Script/Engine.PrimitiveComponent))
      (Variables|Ref|SetDMI _returnvalue))))

(event Collision|EventActorBeginOverlap
  (params (OtherActor :type Actor%20Object%20Reference)))

(event EventTick
  (params (DeltaSeconds :type Float%20%28single-precision%29)))

(fn ConstructionScript
  (bind _returnvalue (Rendering|Material|CreateDynamicMaterialInstance (Variables|Default|GetCube) 0 (Utilities|Array|Get(acopy) (Variables|Default|GetMaterialRef) (Math|Conversions|ToInteger(Boolean) (Variables|Prop|GetCanDisappear))) "None" :!class /Script/Engine.PrimitiveComponent))
  (Variables|Ref|SetDMI _returnvalue))