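; BP_DeadZone is a kill volume that sends the player back to their last checkpoint on overlap.
; It tracks the character and physics ball pawns, updating both references through the Rolly controller's UpdatePlayerPawn delegate.
; Box overlap by the ball stops its movement, transports it to its checkpoint and resets its gravity direction to downward; the character is simply transported.
; Without a valid checkpoint, either pawn reloads Map_Start.
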(event OnComponentBeginOverlap(Box)
  (params (OverlappedComponent :type Primitive%20Component%20Object%20Reference) (OtherActor :type Actor%20Object%20Reference) (OtherComp :type Primitive%20Component%20Object%20Reference) (OtherBodyIndex :type Integer) (bFromSweep :type Boolean) (SweepResult :type Hit%20Result%20Structure%20%28by%20ref%29))
  (bind _physics_ball (Variables|Default|GetPhysics%20Ball))
  (bind _physics_ball_2 (Variables|Default|GetPhysics%20Ball))
  (bind _third_person (Variables|Default|GetThird%20Person))
  (Utilities|FlowControl|Sequence
    (:then_0
      (if (== OtherActor _physics_ball_2)
        (Default|StopBallMovement _physics_ball_2)
        (Utilities|IsValid (Variables|/Game/OriginalAsset/RollingBP/Blueprints/PhysicsBallBP.PhysicsBallBP_C|GetLastCheckPoint _physics_ball_2)
          (:Is%20Valid
            (Default|TransporttoLastCheckPoint _physics_ball)
            (Variables|/Game/OriginalAsset/RollingBP/Blueprints/PhysicsBallBP.PhysicsBallBP_C|SetGravityDirection _physics_ball "0.000000,0.000000,-980.000000"))
          (:Is%20Not%20Valid
            (Game|OpenLevel(byName) "Map_Start")))))
    (:then_1
      (if (== OtherActor _third_person)
        (Utilities|IsValid (Variables|/Game/OriginalAsset/RollingBP/Blueprints/BP_RollyCharacter.BP_RollyCharacter_C|GetLastCheckPoint _third_person)
          (:Is%20Valid
            (Default|TransporttoLastCheckPoint (Variables|Default|GetThird%20Person)))
          (:Is%20Not%20Valid
            (Game|OpenLevel(byName) "Map_Start")))))))

(event Custom|UpdatePlayerPawn_Event
  (params (ThirdPerson :type BP%20Rolly%20Character%20Object%20Reference) (PhysicsBall :type Physics%20Ball%20BP%20Object%20Reference))
  (Variables|Default|SetThird%20Person ThirdPerson)
  (Variables|Default|SetPhysics%20Ball PhysicsBall))

(event EventBeginPlay
  (Utilities|FlowControl|Sequence
    (:then_0
      (bind _asrolly_controller (CallFunction|BFLGetController))
      (bind _output_get (Variables|Ref|SetAs%20Rolly%20Controller _asrolly_controller))
      (EventDispatchers|AssignUpdatePlayerPawn _output_get (delegate Custom|UpdatePlayerPawn_Event)))
    (:then_1
      (bind _asbp_rolly_character (Utilities|Casting|CastToBP_RollyCharacter (Game|Player|GetPlayerPawn 0)))
      (Variables|Default|SetThird%20Person _asbp_rolly_character))))

(event Collision|EventActorBeginOverlap
  (params (OtherActor :type Actor%20Object%20Reference)))

(event EventTick
  (params (DeltaSeconds :type Float%20%28single-precision%29)))

(fn ConstructionScript)